(event `self.ReceiveBeginPlay`
  (bind _tickspersecond (`self.TicksPerSecond`))
  (bind _output_get (set `self.TicksPerSecond` (`KismetMathLibrary.SelectFloat` 60.0 _tickspersecond (== _tickspersecond 0.0))))
  (bind _returnvalue (`KismetSystemLibrary.K2_SetTimer` null "TickSunTime" (/ 1.0 _output_get) true))
  (set `self.SkyUpdateTimer` _returnvalue)
  (if (not (`self.EnableRotationAtBeginning`))
    (`self.StopSkyRotation`)))

(fn `CorrectPositionForRendering`
  (params (ObjectPosition :type "CelestialPosition Structure"))
  (returns (ReturnValue :type "Rotator Structure"))
  ;[1 1 1] Adjust rotation so the Y axis is inverted cause Planet's movement is from East -> West, also displace the Azimuth's North to point to East (+90º).
  (return (`KismetMathLibrary.MakeRotator` 0.0 (* (`OrbitCalculations.IncrementAngleAndLimitTo360` ObjectPosition_Elevation) -1.0) (`OrbitCalculations.IncrementAngleAndLimitTo360` ObjectPosition_Azimuth 90.0))))

(fn `Display Moon`
  (params (ShowMoon :type Boolean))
  (bind _moon (`self.Moon`))
  (bind _starsmaterial (`self.StarsMaterial`))
  (if ShowMoon
    (`SceneComponent.SetVisibility` _moon true false)
    (`MaterialInstanceDynamic.SetScalarParameterValue` _starsmaterial "ShowMoon" 1.0)
    (else
      (`SceneComponent.SetVisibility` _moon false false)
      (`MaterialInstanceDynamic.SetScalarParameterValue` _starsmaterial "ShowMoon" 0.0))))

(fn `DisplayStars`
  (params (ShowStars :type Boolean) (ShowMilkyWay :type Boolean) (ShowConstelations :type Boolean))
  (locals (`ShowMilkyWay?` :type Boolean) (`Show Constelatons?` :type Boolean) (`ShowStars?` :type Boolean))
  (bind _starsmaterial (`self.StarsMaterial`))
  (bind _starsmaterial_2 (`self.StarsMaterial`))
  (bind _starsmaterial_3 (`self.StarsMaterial`))
  (set `local.ShowStars?` ShowStars)
  (set `local.ShowMilkyWay?` ShowMilkyWay)
  (set `local.Show Constelatons?` ShowConstelations)
  (if (`local.ShowStars?`)
    (`MaterialInstanceDynamic.SetScalarParameterValue` _starsmaterial_2 "ShowStars" 1.0)
    (else
      (`MaterialInstanceDynamic.SetScalarParameterValue` _starsmaterial_2 "ShowStars" 0.0)))
  (if (`local.ShowMilkyWay?`)
    (`MaterialInstanceDynamic.SetScalarParameterValue` _starsmaterial_3 "ShowMilkyWay" 1.0)
    (else
      (`MaterialInstanceDynamic.SetScalarParameterValue` _starsmaterial_3 "ShowMilkyWay" 0.0)))
  (if (`local.Show Constelatons?`)
    (`MaterialInstanceDynamic.SetScalarParameterValue` _starsmaterial "ShowConstelations" 1.0)
    (else
      (`MaterialInstanceDynamic.SetScalarParameterValue` _starsmaterial "ShowConstelations" 0.0))))

(fn `DisplaySun`
  (params (ShowSun :type Boolean))
  (bind _sun (`self.Sun`))
  (if ShowSun
    (`SceneComponent.SetVisibility` _sun true false)
    (else
      (`SceneComponent.SetVisibility` _sun false false))))

(fn `GetInGameDate`
  (returns (CurrentDate :type "DateTime Structure"))
  (if (`self.UseSystemTimeInternal`)
    (return (`OrbitCalculations.GetLocalDateTimeFromUtcDateTime` (`KismetMathLibrary.MakeDateTime` (`self.CurrentYear`) (`self.CurrentMonth`) (`self.CurrentDay`) (`self.CurrentHours`) (`self.CurrentMinutes`) (`self.CurrentSeconds`))))
    (else
      (return (`KismetMathLibrary.MakeDateTime` (`self.CurrentYear`) (`self.CurrentMonth`) (`self.CurrentDay`) (`self.CurrentHours`) (`self.CurrentMinutes`) (`self.CurrentSeconds`))))))

(fn `GetMoonPosition`
  (returns (MoonPosition :type "CelestialPosition Structure"))
  (return (`self.MoonPosition`)))

(fn `GetSkyPosition`
  (returns (SkyPosition :type "CelestialPosition Structure"))
  (return (`self.SkyPosition`)))

(fn `GetSunPosition`
  (returns (SunPosition :type "CelestialPosition Structure"))
  (return (`self.SunPosition`)))

(fn `IsDST`
  (params (DSTEnable :type Boolean) (DSTStartMonth :type Integer) (DSTStartDay :type Integer) (DSTEndMonth :type Integer) (DSTEndDay :type Integer) (DSTSwitchHour :type Integer))
  (returns (IsDST :type Boolean))
  (bind _currentyear (`self.CurrentYear`))
  (bind _returnvalue (`KismetMathLibrary.MakeDateTime` (`self.CurrentYear`) (`self.CurrentMonth`) (`self.CurrentDay`) (`self.CurrentHours`) (`self.CurrentMinutes`) (`self.CurrentSeconds`)))
  (return (and DSTEnable (and (>= _returnvalue (`KismetMathLibrary.MakeDateTime` _currentyear DSTStartMonth DSTStartDay DSTSwitchHour)) (<= _returnvalue (`KismetMathLibrary.MakeDateTime` _currentyear DSTEndMonth DSTEndDay DSTSwitchHour))))))

(fn `SetDayTime`
  (params (Hours :type Integer) (Minutes :type Integer) (Seconds :type Integer))
  (bind _output_get (set `self.CurrentHours` Hours))
  (bind _output_get_2 (set `self.CurrentMinutes` Minutes))
  (bind _output_get_3 (set `self.CurrentSeconds` Seconds))
  (set `self.TimeOfDayInSeconds` (`KismetMathLibrary.Conv_IntToDouble` (+ _output_get_3 (* _output_get_2 60) (* _output_get 3600)))))

(fn `SetDST`
  (params (UseDaylightSavingTime :type Boolean) (DSTStartMonth :type Integer) (DSTStartDay :type Integer) (DSTEndMonth :type Integer) (DSTEndDay :type Integer) (DSTSwitchHour :type Integer))
  (`|ExecutionSequence`
    (:`then_0`
      (set `self.UseDaylightSavingTime` UseDaylightSavingTime))
    (:`then_1`
      (set `self.DSTStartMonth` DSTStartMonth))
    (:`then_2`
      (set `self.DSTStartDay` DSTStartDay))
    (:`then_3`
      (set `self.DSTEndMonth` DSTEndMonth))
    (:`then_4`
      (set `self.DSTEndDay` DSTEndDay))
    (:`then_5`
      (set `self.DSTSwitchHour` DSTSwitchHour))))

(fn `SetInGameDate`
  (params (NewDateTime :type "DateTime Structure"))
  (bind (_year _month _day _hour _minute _second) (`KismetMathLibrary.BreakDateTime` NewDateTime))
  (set `self.UseSystemTimeInternal` false)
  (set `self.CurrentYear` _year)
  (set `self.CurrentMonth` _month)
  (set `self.CurrentDay` _day)
  (`self.SetDayTime` _hour _minute _second)
  (`self.UpdateSky`))

(fn `SetLocation`
  (params (Latidude :type "Float (double-precision)") (Longitude :type "Float (double-precision)"))
  (set `self.Latitude` Latidude)
  (set `self.Longitude` Longitude))

(fn `SetTicks`
  (params (Ticks :type Integer))
  (bind _returnvalue (`KismetMathLibrary.Conv_IntToDouble` Ticks))
  (bind _returnvalue_2 (`KismetMathLibrary.SelectFloat` 60.0 _returnvalue (== _returnvalue 0.0)))
  (`KismetSystemLibrary.K2_ClearAndInvalidateTimerHandle` (`self.SkyUpdateTimer`))
  (set `self.TicksPerSecond` _returnvalue_2)
  (bind _returnvalue_3 (`KismetSystemLibrary.K2_SetTimer` null "TickSunTime" (/ 1.0 _returnvalue_2) true))
  (set `self.SkyUpdateTimer` _returnvalue_3))

(fn `SetTimeZone`
  (params (TimeZoneIndex :type Byte))
  (set `self.TimeZone` (cast `/Game/EnhancedSkyMap/E_TimeZones` TimeZoneIndex))
  (`self.UpdateTimeZoneInternal`))

(fn `StartSkyRotation`
  (`KismetSystemLibrary.K2_UnPauseTimerHandle` (`self.SkyUpdateTimer`)))

(fn `StopSkyRotation`
  (`KismetSystemLibrary.K2_PauseTimerHandle` (`self.SkyUpdateTimer`)))

(fn `TickSunTime`
  (bind _output_get (set `self.TimeOfDayInSeconds` (+ (`self.TimeOfDayInSeconds`) (* (`self.SpeedFactor`) (/ 1.0 (`self.TicksPerSecond`))))))
  (`self.UpdateTimeZoneInternal`)
  (bind (_returnvalue_days _returnvalue_hours _returnvalue_minutes _returnvalue_seconds) (`KismetMathLibrary.BreakTimespan` (`KismetMathLibrary.MakeTimespan` 0 0 0 (`KismetMathLibrary.FTrunc` _output_get))))
  (set `self.CurrentHours` _returnvalue_hours)
  (set `self.CurrentMinutes` _returnvalue_minutes)
  (set `self.CurrentSeconds` _returnvalue_seconds)
  (if (>= (`self.TimeOfDayInSeconds`) 86400.0)
    (`self.IncrementDay`) ; Increment day already update the Sun position
    (else
      (`self.UpdateSky`))))

(fn `UpdateSky`
  (bind _stars (`self.Stars`))
  (bind _sun (`self.Sun`))
  (bind _moon (`self.Moon`))
  (bind _isdst (`self.IsDST` (`self.UseDaylightSavingTime`) (`self.DSTStartMonth`) (`self.DSTStartDay`) (`self.DSTEndMonth`) (`self.DSTEndDay`) (`self.DSTSwitchHour`)))
  (`|ExecutionSequence`
    (:`then_1`
      (`/Engine/EditorBlueprintResources/StandardMacros.IsValid` _sun
        (:`Is Valid`
          (switch `EComponentMobility` (`SceneComponent.Mobility` _sun)
            (:`Movable`
              (bind _returnvalue (`OrbitCalculations.GetSunPosition` (`self.Latitude`) (`self.Longitude`) (`self.CurrentYear`) (`self.CurrentMonth`) (`self.CurrentDay`) (`self.CurrentHours`) (`self.CurrentMinutes`) (`self.CurrentSeconds`) (`self.TimeZoneInternal`) _isdst))
              (bind _output_get (set `self.SunPosition` _returnvalue))
              (`SceneComponent.K2_SetRelativeRotation` (`self.Sun`) (`self.CorrectPositionForRendering` _output_get) false false))))))
    (:`then_2`
      (`/Engine/EditorBlueprintResources/StandardMacros.IsValid` _moon
        (:`Is Valid`
          (switch `EComponentMobility` (`SceneComponent.Mobility` _moon)
            (:`Movable`
              (bind _returnvalue_2 (`OrbitCalculations.GetMoonPosition` (`self.Latitude`) (`self.Longitude`) (`self.CurrentYear`) (`self.CurrentMonth`) (`self.CurrentDay`) (`self.CurrentHours`) (`self.CurrentMinutes`) (`self.CurrentSeconds`) (`self.TimeZoneInternal`) _isdst))
              (bind _output_get_2 (set `self.MoonPosition` _returnvalue_2))
              (`SceneComponent.K2_SetRelativeRotation` (`self.Moon`) (`self.CorrectPositionForRendering` _output_get_2) false false))))))
    (:`then_3`
      (`/Engine/EditorBlueprintResources/StandardMacros.IsValid` _stars
        (:`Is Valid`
          (switch `EComponentMobility` (`SceneComponent.Mobility` _stars)
            (:`Static`
              _)
            (:`Stationary`
              _)
            (:`Movable`
              ;[1 0.3997 0.9134] We are only simulating approximate sky position here, because we don't render star by star
              (bind _returnvalue_3 (`OrbitCalculations.GetSkyPosition` (`self.Latitude`) (`self.Longitude`) (`self.CurrentYear`) (`self.CurrentMonth`) (`self.CurrentDay`) (`self.CurrentHours`) (`self.CurrentMinutes`) (`self.CurrentSeconds`) (`self.TimeZoneInternal`) _isdst))
              (bind _output_get_3 (set `self.SkyPosition` _returnvalue_3))
              (bind (_returnvalue_roll _returnvalue_pitch _returnvalue_yaw) (`KismetMathLibrary.BreakRotator` (`OrbitCalculations.GetRotatorForSky` _output_get_3)))
              (`SceneComponent.K2_SetRelativeRotation` (`self.Stars`) (`KismetMathLibrary.MakeRotator` (- _returnvalue_roll 90.0) (- _returnvalue_pitch 90.0) _returnvalue_yaw) false false)
              (`self.SkyMoved` (`self.GetInGameDate`) (`self.SunPosition`) (`self.MoonPosition`) (`self.SkyPosition`))))
          (return))))))

(fn `UserConstructionScript`
  (bind _startingyear (`self.StartingYear`))
  (bind _returnvalue (`KismetMathLibrary.DaysInMonth` _startingyear (`self.StartingMonth`)))
  ;[0.3873 0.4415 1] Date and Time initialization
  (set `self.CurrentYear` _startingyear) ; Initialize current date
  (if (> (`self.StartingDay`) _returnvalue)
    (set `self.StartingDay` _returnvalue))
  (set `self.CurrentMonth` (`self.StartingMonth`))
  (set `self.CurrentDay` (`self.StartingDay`))
  (if (`self.UseSystemTime (override)`)
    (`self.SetupUseSystemTime`)
    (`self.UpdateTimeZoneInternal` :!label _label)
    ;[0.4773 1 0.4503] Sky Update
    (`self.SetDayTime` (`self.CurrentHours`) (`self.CurrentMinutes`) (`self.CurrentSeconds`))
    (`self.UpdateSky`)
    ;[0.935 0.5647 1] Material Instance for Stars
    (bind _returnvalue_2 (`PrimitiveComponent.CreateDynamicMaterialInstance` (`self.Stars`) 0 "/Game/EnhancedSkyMap/MI_SkyStarsDemo.MI_SkyStarsDemo" "None"))
    (set `self.StarsMaterial` _returnvalue_2)
    (else
      (`|ExecutionSequence`
        (:`then_0`
          (set `self.CurrentHours` (`self.StartingHours`)))
        (:`then_1`
          (set `self.CurrentMinutes` (`self.StartingMinutes`)))
        (:`then_2`
          (set `self.CurrentSeconds` (`self.StartingSeconds`)))
        (:`then_3`
          (goto _label))))))

(fn `UseSystemTime`
  (params (`Use System Time` :type Boolean))
  (set `self.UseSystemTime (override)` `Use System Time`)
  (`self.SetupUseSystemTime`)
  (`self.UpdateSky`))